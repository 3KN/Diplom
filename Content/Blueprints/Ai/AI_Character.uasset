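; AI_Character is an enemy Blueprint with logic for tracking kills and ending the game on a win.
; Its kill logic, currently not triggered by any event, increments the ThirdPersonCharacter's KillCount, destroys the enemy, and sets a win message when that count equals the game mode's Enemies.
; EndGame pauses the game, shows the mouse cursor and displays the GameEnd widget.
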(fn `EndGame`
  (bind _returnvalue (`GameplayStatics.GetPlayerController` 0))
  (`GameplayStatics.SetGamePaused` true)
  (set `PlayerController.bShowMouseCursor` true _returnvalue)
  (bind _returnvalue_2 (`|CreateWidget` "/Game/Blueprints/HUD/GameEnd.GameEnd_C" _returnvalue))
  (`UserWidget.AddToViewport` _returnvalue_2 0))

(fn `UserConstructionScript`)