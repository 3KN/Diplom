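; EnemyContext is an EQS context that supplies the querier's enemy as a single actor for environment queries.
; For AI-controlled queriers, it reads the Enemy variable from the Runner_AI controller.
; When the querier is an EQS testing pawn, it substitutes the first ThirdPersonCharacter found in the world, so queries can be tested without that controller.
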(fn `ProvideSingleActor`
  (params (QuerierObject :type "Object Object Reference") (QuerierActor :type "Actor Object Reference"))
  (returns (ResultingActor :type "Actor Object Reference"))
  (locals (TempEnemy :type "Actor Object Reference") (NewLocalVar_0 :type "Actor Object Reference"))
  (bind _returnvalue (`AIBlueprintHelperLibrary.GetAIController` QuerierActor))
  (cast `EQSTestingPawn` QuerierActor
    (:`then`
      (bind _outactors (`GameplayStatics.GetAllActorsOfClass` "/Game/ThirdPersonBP/Blueprints/ThirdPersonCharacter.ThirdPersonCharacter_C"))
      (set `local.TempEnemy` (`|GetArrayItem` _outactors)))
    (:`CastFailed`
      (if (!= _returnvalue null)
        (bind _asrunner_ai (cast `/Game/Blueprints/Ai/Runner_AI` _returnvalue)
          (:`then`
            (set `local.TempEnemy` (`/Game/Blueprints/Ai/Runner_AI.Enemy` _asrunner_ai)))
          (:`CastFailed`
            _)))))
  (return (`local.TempEnemy`)))