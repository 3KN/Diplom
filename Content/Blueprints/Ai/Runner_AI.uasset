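; AI controller for the Runner enemy that runs the Runner_BT behavior tree and treats the first player's pawn as its enemy.
; Shortly after BeginPlay it stores that pawn as the enemy in the Blackboard.
; AIPerception updates involving the enemy refresh a Blackboard visibility flag from the success of the first last-sensed stimulus entry, as does setting a new enemy.
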(event `self.ReceiveBeginPlay`
  (`self.RunBehaviorTree` "/Game/Blueprints/Ai/Runner_BT.Runner_BT")
  (`KismetSystemLibrary.Delay` 0.1)
  (`self.setEnemy` (`GameplayStatics.GetPlayerPawn` 0)))

(event `self.AIPerception.OnPerceptionUpdated`
  (params (UpdatedActors :type "Array of Actor Object Reference"))
  (for _array_element UpdatedActors
    (if (== _array_element (`self.Enemy`))
      (`self.UpdateEnemyBlackboardsKeys` (`self.AIPerception`) _array_element))))

(fn `setEnemy`
  (params (NewEnemy :type "Actor Object Reference"))
  (if (!= NewEnemy (`self.Enemy`))
    (bind _output_get (set `self.Enemy` NewEnemy))
    (`BlackboardComponent.SetValueAsObject` (`AIBlueprintHelperLibrary.GetBlackboard` null) (`self.BlackboardKeyEnemy`) _output_get)
    (`self.UpdateEnemyBlackboardsKeys` (`self.AIPerception`) (`self.Enemy`))))

(fn `UpdateEnemyBlackboardsKeys`
  (params (PerceptionComponent :type "AIPerceptionComponent Object Reference") (EnemyActor :type "Actor Object Reference"))
  (bind _info (`AIPerceptionComponent.GetActorsPerception` PerceptionComponent EnemyActor))
  (`BlackboardComponent.SetValueAsBool` (`AIBlueprintHelperLibrary.GetBlackboard` null) (`self.BlackboardKeyIsEnemyVisible`) (`.bSuccessfullySensed` (break `AIStimulus` (`|GetArrayItem` (`.LastSensedStimuli` (break `ActorPerceptionBlueprintInfo` _info)))))))

(fn `UserConstructionScript`)